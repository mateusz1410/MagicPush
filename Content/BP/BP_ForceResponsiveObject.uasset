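; BP_ForceResponsiveObject is an actor whose mesh reacts to force events, picking its material at BeginPlay from a heavy flag exposed through IsHeavy.
; ApplyForce pushes away from an origin and ApplyForcewithDirection along a given vector, both enabling physics and adding a mass-independent velocity impulse.
; ResetForceObject stops simulation, moves the actor to the mesh's location and reattaches the mesh to the root, since simulating physics detaches it.
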(event EventBeginPlay
  (Rendering|Material|SetMaterial (Variables|Default|GetSM_Object) 0 (select (Variables|Default|GetisHeavyObject) "/Game/BP/M_ForceActive.M_ForceActive" "/Game/BP/MI_ForceActive_Grab.MI_ForceActive_Grab")))

(event Collision|EventActorBeginOverlap
  (params (OtherActor :type Actor%20Object%20Reference)))

(event EventTick
  (params (DeltaSeconds :type Float%20%28single-precision%29)))

(event EventApplyForce
  (params (forceOrigin :type Vector :default "0, 0, 0") (power :type Float%20%28single-precision%29))
  (bind _sm_object (Variables|Default|GetSM_Object))
  (Physics|SetSimulatePhysics _sm_object true)
  (Physics|AddImpulse _sm_object (* (Math|Vector|Normalize (- (Transformation|GetWorldLocation (Variables|Default|GetSM_Object)) forceOrigin)) power) "None" true))

(event EventApplyForcewithDirection
  (params (directionVector :type Vector :default "0, 0, 0") (power :type Float%20%28single-precision%29))
  (bind _sm_object (Variables|Default|GetSM_Object))
  (Physics|SetSimulatePhysics _sm_object true)
  (Physics|AddImpulse _sm_object (* directionVector power) "None" true))

(event EventResetForceObject
  (bind _sm_object (Variables|Default|GetSM_Object))
  (if (Physics|IsSimulatingPhysics _sm_object "None")
    (Physics|SetSimulatePhysics _sm_object false)
    (Transformation|SetActorLocation (Transformation|GetWorldLocation _sm_object) false false)
    (Transformation|AttachComponentToComponent (Variables|Default|GetSM_Object) (Variables|Default|GetDefaultSceneRoot) "None" "KeepWorld" "KeepWorld" "KeepWorld" true)))

(fn ConstructionScript)

(fn IsHeavy
  (return (Variables|Default|GetisHeavyObject)))